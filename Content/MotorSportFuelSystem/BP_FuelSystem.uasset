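; Vehicle fuel system that drains a main tank, then a hidden reserve, based on engine load from the referenced movement component.
; After initialization, a self-rescheduling one-second timer subtracts consumption derived from engine RPM, injection time, nozzle performance and cylinder count.
; RepNotify handlers on both fuel levels set the empty flags that switch draining to the reserve and stop the timer when it runs out.
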(event `Initialize_Vehicle`
  (params (Movement :type "WheeledVehicleMovementComponent Object Reference") (Vehicle :type "/Game/MotorSportFuelSystem/BP_Vehicle Object Reference"))
  ;[1 0.12 0.12] Initialize vehicle
  (`self.InitializeVehicle` Movement Vehicle)
  (`self.FuelConsumptionTimer`))

(event `self.ReceiveBeginPlay`
  ;[0.781 1 0.4225] Set variables defaults
  (set `self.FuelTankSize` (`self.MaxFuelTankSize`))
  (set `self.HiddenFuel` (`self.MaxHiddenFuel`)))

(fn `CalculateFuelTankConsumption`
  (set `self.FuelTankSize` (- (`self.FuelTankSize`) (`self.M_FuelConsumption`)))
  (`self.FuelConsumptionTimer`))

(fn `CalculateHiddenFuelConsumption`
  (set `self.HiddenFuel` (- (`self.HiddenFuel`) (`self.M_FuelConsumption`)))
  (`self.FuelConsumptionTimer`))

(fn `FuelConsumptionTimer`
  (if (not (`self.FuelIsOver`))
    (if (not (`self.FuelTankIsEmpty`))
      (`KismetSystemLibrary.K2_SetTimer` null "CalculateFuelTankConsumption" 1.0)
      (else
        (`KismetSystemLibrary.K2_SetTimer` null "CalculateHiddenFuelConsumption" 1.0)))))

(fn `FuelPerMinute`
  (returns (FuelPreMinute :type "Float (double-precision)"))
  (return (* (* (* (/ (`self.InjectionTime`) 60000.0) (`self.NozzlePerformance`)) (/ (`WheeledVehicleMovementComponent.GetEngineRotationSpeed` (`self.MovementReference`)) 2.0)) (`KismetMathLibrary.Conv_IntToDouble` (`self.CylindersCount`)))))

(fn `GetFuelIsOver`
  (returns (FuelIsOver :type Boolean))
  (return (`self.FuelIsOver`)))

(fn `GetFuelTankSize`
  (returns (FuelSize :type "Float (double-precision)"))
  (return (`self.FuelTankSize`)))

(fn `GetHiddenFuel`
  (returns (HiddenFuel :type "Float (double-precision)"))
  (return (`self.HiddenFuel`)))

(fn `InitializeVehicle`
  (params (Movement :type "WheeledVehicleMovementComponent Object Reference") (Vehicle :type "/Game/MotorSportFuelSystem/BP_Vehicle Object Reference"))
  (set `self.MovementReference` Movement)
  (set `self.VehicleReference` Vehicle))

(fn `OnRep_FuelTankSize`
  (if (<= (`self.FuelTankSize`) 0.0)
    (set `self.FuelTankIsEmpty` true)
    (else
      (set `self.FuelTankIsEmpty` false))))

(fn `OnRep_HiddenFuel`
  (if (<= (`self.HiddenFuel`) 0.0)
    (set `self.FuelIsOver` true)
    (else
      (set `self.FuelIsOver` false))))